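; BP_VoyagerARController is a controller for the Voyage AR project that manages object customization UI.
; It creates, initializes, stores and removes two widgets: a general user customization panel and a texture-change panel.
; The texture panel gets an event binding for returning a selection to the controller.
; SendTextureToCharacter rebroadcasts a texture through the OnSetTextureForObject dispatcher, keeping UI decoupled from the object that applies it.
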(event EventBeginPlay)

(event EventTick
  (params (DeltaSeconds :type Float%20%28single-precision%29)))

(fn ConstructionScript)

(fn ShowCustomizationUI
  (params (Params :type Available%20Customization%20Params%20Structure))
  (bind _returnvalue (UserInterface|CreateWidget "/Game/VoyageARDevelop/Widgets/W_UserCustomizationBase.W_UserCustomizationBase_C"))
  (UserInterface|Viewport|AddtoViewport _returnvalue 0)
  (Default|Init _returnvalue Params)
  (Variables|Default|SetCustomizationWidget _returnvalue))

(fn RemoveCustomixationUI
  (Widget|RemovefromParent (Variables|Default|GetCustomizationWidget)))

(fn ShowSetTextureUI
  (params (NewParam :type Array%20of%20Texture%202D%20Object%20References))
  (bind _returnvalue (UserInterface|CreateWidget "/Game/VoyageARDevelop/Widgets/W_ChangeTextureBase.W_ChangeTextureBase_C"))
  (Default|Init _returnvalue NewParam)
  (UserInterface|Viewport|AddtoViewport _returnvalue 0)
  (EventDispatchers|BindEventtoSendTexturetoController _returnvalue (EventDispatchers|CreateEvent :!event SendTexturetoCharacter))
  (Variables|Default|SetCustomizationTextureWidget _returnvalue))

(fn RemoveSetTextureUI
  (Widget|RemovefromParent (Variables|Default|GetCustomizationTextureWidget)))

(fn SendTexturetoCharacter
  (params (Texture :type Texture%202D%20Object%20Reference))
  (Default|CallOnSetTextureforObject Texture))